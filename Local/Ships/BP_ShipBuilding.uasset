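; Placeable building piece for a ship, which can later be launched as an actual ship actor.
; CanBePlaced extends the parent placement check with a box trace at WaterCheckBox, failing unless the hit actor is water deep enough for the ship.
; LaunchShip runs only on the server for visible non-brush instances, spawning ShipClass at the building's location and rotation, calling DoLaunch, then destroying the building.
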(event Custom|LaunchShip
  (if (Math|Boolean|ANDBoolean (Networking|IsServer) (not (Variables|Default|GetIsABrush)) (not (Variables|Default|GetbHidden)))
    (bind _returnvalue (Game|SpawnActorfromClass (Variables|Default|GetshipClass) (Math|Transform|MakeTransform (Transformation|GetActorLocation) (Transformation|GetActorRotation) "1.000000,1.000000,1.000000") "AlwaysSpawn" 0 0))
    (Variables|/Game/Mods/ShipsOfTheExiled/Ships/BP_Ship.BP_Ship_C|SetcurrentMode _returnvalue "NewEnumerator0")
    (Default|DoLaunch _returnvalue self)
    (Actor|DestroyActor)))

(fn ConstructionScript
  (|CallParentFunction))

(fn CanbePlaced
  (params (AttachTo :type Buildable%20Base%20Object%20Reference) (InstanceIndex :type Integer))
  (bind _watercheckbox (Variables|Default|GetWaterCheckBox))
  (bind _returnvalue (Transformation|GetWorldLocation _watercheckbox))
  (bind (_x _y _z) (Math|Vector|BreakVector _returnvalue))
  (bind (_failedmessage _returnvalue_2) (|CallParentFunction AttachTo InstanceIndex))
  (if (or (Utilities|Enum|Equal(Enum) _returnvalue_2 "Success") (Utilities|Enum|Equal(Enum) _returnvalue_2 "Success_Update"))
    (bind _outhit (Class|KismetSystemLibrary|BoxTraceSingleforObjects _returnvalue (Math|Vector|MakeVector _x _y (- _z 1.0)) (Components|Box|GetScaledBoxExtent _watercheckbox) (Transformation|GetWorldRotation _watercheckbox) (Utilities|Array|MakeArray "ObjectTypeQuery12") false 0 "ForOneFrame" true))
    (bind _out_is_water (CallFunction|IsWater (.HitActor (Collision|BreakHitResult _outhit))))
    (if _out_is_water
      (return "" "Success")
      (else
        (return "Ship must be placed in deep enough water" "Fail")))
    (else
      (return _failedmessage _returnvalue_2))))