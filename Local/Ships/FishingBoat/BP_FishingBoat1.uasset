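; BP_FishingBoat1 is a fishing boat Blueprint that cycles its sail through random colours.
; On BeginPlay, except on dedicated servers, it creates a dynamic sail material and applies it to instanced static mesh components using the sailcloth_sm mesh.
; A fast looping timer, started when a sail is found, randomizes the material's tint parameter locally, with no replication.
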(event Custom|changeSailColor
  (Rendering|Material|SetVectorParameterValue (Variables|Default|GetsailMaterial) "tint" (Utilities|Struct|MakeLinearColor (Math|Random|RandomFloat) (Math|Random|RandomFloat) (Math|Random|RandomFloat) 1.0) :!class /Script/Engine.MaterialInstanceDynamic))

(event EventBeginPlay
  (|CallParentFunction)
  (if (not (Networking|IsDedicatedServer))
    (bind _returnvalue (Rendering|Material|CreateDynamicMaterialInstance "/Game/Mods/ShipsOfTheExiled/Assets/fishing_boat_pack/materials/mat_sail.mat_sail" :!class /Script/Engine.KismetMaterialLibrary))
    (Variables|Default|SetsailMaterial _returnvalue)
    (for _array_element (Actor|GetComponentsByClass "/Script/Engine.InstancedStaticMeshComponent")
      (if (Utilities|Enum|Equal(Enum) (Utilities|GetDisplayName (Variables|/Script/Engine.StaticMeshComponent|GetStaticMesh _array_element)) "sailcloth_sm")
        (Rendering|Material|SetMaterial _array_element 0 (Variables|Default|GetsailMaterial))
        (Utilities|Time|SetTimerbyEvent (delegate Custom|changeSailColor) 0.1 true)))))

(fn ConstructionScript
  (|CallParentFunction))