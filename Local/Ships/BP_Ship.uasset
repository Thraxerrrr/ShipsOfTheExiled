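; Persistent Conan Exiles ship whose hull is copied from a building's instanced meshes and rebuilt from saved mesh paths and transforms.
; A server overlap timer and hit events attach placeables to the hull and give characters passenger components.
; Collision boxes flag obstacles ahead and behind, while non-dedicated instances animate eased bobbing and splash particles on Tick.
; It also supplies the steering socket, forwards the radial menu to its control component, and handles scuttling.
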(event OnComponentBeginOverlap(AheadCollisionBox)
  (params (OverlappedComponent :type Primitive%20Component%20Object%20Reference) (OtherActor :type Actor%20Object%20Reference) (OtherComp :type Primitive%20Component%20Object%20Reference) (OtherBodyIndex :type Integer) (bFromSweep :type Boolean) (SweepResult :type Hit%20Result%20Structure%20%28by%20ref%29))
  ;[1 1 1] Collision ahead/behind
  (if (CallFunction|IsObstacle OtherActor)
    (Variables|Default|SetoverlapObstacleAhead true)))

(event OnComponentBeginOverlap(BehindCollisionBox)
  (params (OverlappedComponent :type Primitive%20Component%20Object%20Reference) (OtherActor :type Actor%20Object%20Reference) (OtherComp :type Primitive%20Component%20Object%20Reference) (OtherBodyIndex :type Integer) (bFromSweep :type Boolean) (SweepResult :type Hit%20Result%20Structure%20%28by%20ref%29))
  ;[1 1 1] Collision ahead/behind
  (if (CallFunction|IsObstacle OtherActor)
    (Variables|Default|SetoverlapObstacleBehind true)))

(event OnComponentEndOverlap(BehindCollisionBox)
  (params (OverlappedComponent :type Primitive%20Component%20Object%20Reference) (OtherActor :type Actor%20Object%20Reference) (OtherComp :type Primitive%20Component%20Object%20Reference) (OtherBodyIndex :type Integer))
  ;[1 1 1] Collision ahead/behind
  (Variables|Default|SetoverlapObstacleBehind (CallFunction|IsAnyObstacle (Collision|GetOverlappingActors (Variables|Default|GetBehindCollisionBox) 0 :!class /Script/Engine.PrimitiveComponent))))

(event OnComponentEndOverlap(AheadCollisionBox)
  (params (OverlappedComponent :type Primitive%20Component%20Object%20Reference) (OtherActor :type Actor%20Object%20Reference) (OtherComp :type Primitive%20Component%20Object%20Reference) (OtherBodyIndex :type Integer))
  ;[1 1 1] Collision ahead/behind
  (Variables|Default|SetoverlapObstacleAhead (CallFunction|IsAnyObstacle (Collision|GetOverlappingActors (Variables|Default|GetAheadCollisionBox) 0 :!class /Script/Engine.PrimitiveComponent))))

(event Custom|ProcessCharacterOverlap
  (params (character :type Base%20BP%20Char%20Object%20Reference))
  ;[0 0.07858 1] Overlapping Placeables and Characters
  (if (not (Utilities|IsValid (Actor|GetComponentbyClass character "/Game/Mods/ShipsOfTheExiled/System/BP_ShipPassengerComp.BP_ShipPassengerComp_C")))
    (bind _returnvalue (Class|FuncomGenericLibrary|AddComponentbyClass character "/Game/Mods/ShipsOfTheExiled/System/BP_ShipPassengerComp.BP_ShipPassengerComp_C" (Math|Conversions|ToTransform(Vector) "0, 0, 0")))
    (Variables|/Game/Mods/ShipsOfTheExiled/System/BP_ShipPassengerComp.BP_ShipPassengerComp_C|Setship (.AsBP%20Ship%20Passenger%20Comp (Utilities|Casting|CastToBP_ShipPassengerComp _returnvalue)) self)))

(event Custom|toggleBobbing
  ;[0.2165 1 0.2923] Bobbing and water splash effects
  (bind _output_get (Variables|Default|SetbobbingEnabled (not (Variables|Default|GetbobbingEnabled))))
  (if (not _output_get)
    (Utilities|FlowControl|Delay 1.0)
    (CallFunction|MulticastResetBobbing)))

(event Custom|TimedCheckOverlaps
  ;[0.6178 1 0] BeginPlay
  (for _array_element (CallFunction|CheckforOverlappingActors)
    (CallFunction|ProcessActorOverlap _array_element)))

(event Custom|ProcessActorOverlap
  (params (actor :type Actor%20Object%20Reference))
  ;[0 0.07858 1] Overlapping Placeables and Characters
  (bind _asbp_master_placeables (Utilities|Casting|CastToBP_Master_Placeables actor)
    (:then
      (CallFunction|ProcessPlaceableOverlap _asbp_master_placeables))
    (:CastFailed
      (bind _asbase_bpchar (Utilities|Casting|CastToBaseBPChar actor))
      (CallFunction|ProcessCharacterOverlap _asbase_bpchar))))

(event Custom|MulticastResetBobbing
  ;[0.2165 1 0.2923] Bobbing and water splash effects
  (Transformation|SetRelativeRotation (Variables|Default|GetMesh) "0, 0, 0" false false))

(event Custom|scuttle
  ;[1 0.04025 0.09001] Scuttling
  (Class|PersistenceComponent|Delete (Variables|Default|GetActorPersistence))
  (Utilities|FlowControl|Sequence
    (:then_0
      (for _array_element (Actor|GetAttachedActors)
        (bind _asbp_master_placeables (Utilities|Casting|CastToBP_Master_Placeables _array_element))
        (Actor|DestroyActor _asbp_master_placeables)))
    (:then_1
      (Actor|DestroyActor))))

(event Custom|ProcessPlaceableOverlap
  (params (placeable :type BP%20Master%20Placeables%20Object%20Reference))
  (bind _conanbuildingpersistence (Variables|/Game/Systems/Building/Placeables/BP_Master_Placeables.BP_Master_Placeables_C|GetConanBuildingPersistence placeable))
  (bind _returnvalue (Class|PersistenceComponent|GetUniqueID _conanbuildingpersistence))
  (bind _returnvalue_2 (Class|DreamworldBlueprints|ToString(UniqueID) _returnvalue))
  ;[0 0.07858 1] Overlapping Placeables and Characters
  (if (and (not (Utilities|IsValid (Variables|/Game/Mods/ShipsOfTheExiled/System/SOTE_Placeable_AC.SOTE_Placeable_AC_C|Getship (Actor|GetComponentbyClass placeable "/Game/Mods/ShipsOfTheExiled/System/SOTE_Placeable_AC.SOTE_Placeable_AC_C")))) (Utilities|IsValid _conanbuildingpersistence))
    (if (== (Utilities|Array|FindItem (Variables|Default|GetknownPlaceables) _returnvalue_2) -1)
      (Utilities|Array|Add (Variables|Default|GetknownPlaceables) _returnvalue_2)
      (Transformation|AttachComponentToComponent placeable (Variables|Default|GetMesh) "None" "KeepWorld" "KeepWorld" "KeepWorld" true)
      (Variables|/Game/Mods/ShipsOfTheExiled/System/SOTE_Placeable_AC.SOTE_Placeable_AC_C|Setship (Actor|GetComponentbyClass placeable "/Game/Mods/ShipsOfTheExiled/System/SOTE_Placeable_AC.SOTE_Placeable_AC_C") self)
      (Development|PrintString (Utilities|String|Append "Attached placeable: " (Utilities|GetDisplayName placeable)) true true "(R=0.000000,G=0.660000,B=1.000000,A=1.000000)" 6.0))))

(event EventBeginPlay
  ;[0.6178 1 0] BeginPlay
  (|CallParentFunction)
  (if (Networking|IsServer)
    (Utilities|FlowControl|Sequence
      (:then_0
        ;;[1 1 1] Initialize persistence ID
        (if (not (Class|DreamworldBlueprints|IsValidID (Class|PersistenceComponent|GetUniqueID (Variables|Default|GetActorPersistence))))
          (bind _returnvalue (Class|UniqueID|GenerateUniqueID))
          (Class|DreamworldBlueprints|SetUniqueID self _returnvalue)
          (Class|PersistenceComponent|SetDirty (Variables|Default|GetActorPersistence) true 5.0)))
      (:then_1
        (CallFunction|OnRepBuildingInstance) ; If this pawn was just created, make sure it initializes the building instances
      )
      (:then_2
        (Utilities|Time|SetTimerbyEvent (delegate Custom|TimedCheckOverlaps) 2.0 true) ; Keep checking for new placeable/thrall overlaps
      ))))

(event EventEndPlay
  (params (EndPlayReason :type EEndPlayReason%20Enum :default "Destroyed"))
  ;[1 1 1] Needed to prevent crash: "Failed to destroy physics state"
  (for _array_element (Actor|GetComponentsByClass "/Script/Engine.InstancedStaticMeshComponent")
    (Components|DestroyComponent _array_element)))

(event EventTick
  (params (DeltaSeconds :type Float%20%28single-precision%29))
  (bind _rotator (CallFunction|BobbingGetCurrentRotator))
  ;[0.2165 1 0.2923] Bobbing and water splash effects
  (if (not (Networking|IsDedicatedServer))
    (Utilities|FlowControl|Sequence
      (:then_0
        (if (Utilities|IsValid (Variables|Default|GetsteeringCharComp))
          (CallFunction|ToggleWaterSplashParticles (> (Math|Vector|VectorLength (Transformation|GetVelocity (Actor|GetAttachParentActor))) 0.0))
          (Utilities|IsValid+Branch (Pawn|GetController (Variables|/Game/Mods/ShipsOfTheExiled/System/BP_SteeringCharComp.BP_SteeringCharComp_C|GetsteeringChar (Variables|Default|GetsteeringCharComp))) true
            (:True
              (Variables|Default|SetoverlappingWater false)
              (for _array_element (CallFunction|GetOverlappingObjects (Variables|Default|GetWaterCollisionBox) (Utilities|Array|MakeArray "ObjectTypeQuery12"))
                (bind _out_is_water (CallFunction|IsWater (.HitActor (Collision|BreakHitResult _array_element))))
                (Variables|Default|SetoverlappingWater _out_is_water))))))
      (:then_1
        (if (Variables|Default|GetbobbingEnabled)
          (CallFunction|BobbingAdvanceValues DeltaSeconds)
          (Transformation|SetRelativeRotation (Variables|Default|GetMesh) _rotator false false)
          (if (Utilities|IsValid (Variables|Default|GetsteeringCharComp))
            (Default|RepositionSteeringChar (Variables|Default|GetsteeringCharComp) _rotator)))))))

(event EventInteractableMenu
  (params (RadialMenu :type Radial%20Menu%20Object%20Reference) (HitIndex :type Integer))
  ;[1 1 1] Radial Menu
  (Default|BuildInteractableMenu (Variables|Default|GetSOTE_ShipControl_AC) RadialMenu))

(event Collision|EventHit
  (params (MyComp :type Primitive%20Component%20Object%20Reference) (Other :type Actor%20Object%20Reference) (OtherComp :type Primitive%20Component%20Object%20Reference) (bSelfMoved :type Boolean) (HitLocation :type Vector :default "0, 0, 0") (HitNormal :type Vector :default "0, 0, 0") (NormalImpulse :type Vector :default "0, 0, 0") (Hit :type Hit%20Result%20Structure%20%28by%20ref%29))
  ;[0 0.07858 1] Overlapping Placeables and Characters
  (CallFunction|ProcessActorOverlap Other))

(fn ConstructionScript)

(fn OnRepBuildingInstance
  (bind _buildinginstance (Variables|Default|GetbuildingInstance))
  (bind (_meshnames _transforms) (Utilities|Struct|BreakSTRUCT_Ship_BuildingInstance _buildinginstance))
  (for (_array_element _array_index) _meshnames
    (bind _ism (CallFunction|GetorCreateISM _array_element))
    (Components|InstancedStaticMesh|AddInstance _ism (Utilities|Array|Get(acopy) _transforms _array_index))))

(fn UpdateBuildingInstance
  (bind _tmpinstance (LocalVariables|GettmpInstance))
  (bind (_meshnames _transforms) (Utilities|Struct|BreakSTRUCT_Ship_BuildingInstance _tmpinstance))
  (for _array_element (Actor|GetComponentsByClass "/Script/Engine.InstancedStaticMeshComponent")
    (for _index (range 0 (- (Components|InstancedStaticMesh|GetInstanceCount _array_element) 1))
      (Utilities|Array|Add _meshnames (Class|KismetSystemLibrary|GetPathName (Variables|/Script/Engine.StaticMeshComponent|GetStaticMesh _array_element)))
      (Utilities|Array|Add _transforms (.OutInstanceTransform (Components|InstancedStaticMesh|GetInstanceTransform _array_element _index false)))))
  (Variables|Default|SetbuildingInstance (LocalVariables|GettmpInstance))
  (Class|PersistenceComponent|SetDirty (Variables|Default|GetActorPersistence) true 5.0))

(fn GetorCreateISM
  (params (meshName :type String))
  (for _array_element (Actor|GetComponentsByClass "/Script/Engine.InstancedStaticMeshComponent")
    (if (Utilities|Enum|Equal(Enum) (Class|KismetSystemLibrary|GetPathName (Variables|/Script/Engine.StaticMeshComponent|GetStaticMesh _array_element)) meshName)
      (return _array_element)))
  (bind _returnvalue (Class|FuncomGenericLibrary|AddComponentbyClass self "/Script/Engine.InstancedStaticMeshComponent" (Math|Conversions|ToTransform(Vector) "0, 0, 0")))
  (Transformation|AttachComponentToComponent (.AsInstanced%20Static%20Mesh%20Component (Utilities|Casting|CastToInstancedStaticMeshComponent _returnvalue)) (Variables|Default|GetMesh) "None" "KeepWorld" "KeepWorld" "KeepWorld" false) ; Welding sim bodies causes a crash on exit?!
  (bind _returnvalue_2 (Class|FuncomGenericLibrary|LoadAssetfromPath meshName))
  (Components|StaticMesh|SetStaticMesh (.AsInstanced%20Static%20Mesh%20Component (Utilities|Casting|CastToInstancedStaticMeshComponent _returnvalue)) (.AsStatic%20Mesh (Utilities|Casting|CastToStaticMesh _returnvalue_2)))
  (Class|ActorComponent|SetIsReplicated (.AsInstanced%20Static%20Mesh%20Component (Utilities|Casting|CastToInstancedStaticMeshComponent _returnvalue)) true)
  (Collision|SetCollisionObjectType (.AsInstanced%20Static%20Mesh%20Component (Utilities|Casting|CastToInstancedStaticMeshComponent _returnvalue)) "ECC_GameTraceChannel4")
  (return (.AsInstanced%20Static%20Mesh%20Component (Utilities|Casting|CastToInstancedStaticMeshComponent _returnvalue))))

(fn CopyfromBuilding
  (params (building :type Building%20Base%20Object%20Reference))
  (Utilities|FlowControl|Sequence
    (:then_0
      ;[1 1 1] Copy all InstancedStaticMesh components
      (for _array_element (Actor|GetComponentsByClass building "/Script/Engine.InstancedStaticMeshComponent")
        (if (not (Variables|/Script/Engine.SceneComponent|GetbHiddenInGame _array_element))
          (bind _returnvalue (Class|FuncomGenericLibrary|AddComponentbyClass self "/Script/Engine.InstancedStaticMeshComponent" (Transformation|GetRelativeTransform _array_element)))
          (bind _asinstanced_static_mesh_component (Utilities|Casting|CastToInstancedStaticMeshComponent _returnvalue))
          (Transformation|AttachComponentToComponent _asinstanced_static_mesh_component (Variables|Default|GetMesh) "None" "KeepWorld" "KeepWorld" "KeepWorld" false)
          (Class|ActorComponent|SetIsReplicated _asinstanced_static_mesh_component true)
          (Components|StaticMesh|SetStaticMesh _asinstanced_static_mesh_component (Variables|/Script/Engine.StaticMeshComponent|GetStaticMesh _array_element))
          (Collision|SetCollisionObjectType _asinstanced_static_mesh_component "ECC_GameTraceChannel4")
          ;[1 1 1] Copy all instances
          (for _index (range 0 (- (Components|InstancedStaticMesh|GetInstanceCount _array_element) 1))
            (Components|InstancedStaticMesh|AddInstance _asinstanced_static_mesh_component (.OutInstanceTransform (Components|InstancedStaticMesh|GetInstanceTransform _array_element _index false)))))))
    (:then_1
      (Variables|Default|SetownerUUID (Variables|/Script/ConanSandbox.BuildableBase|GetOwnerUniqueID building)))
    (:then_2
      (CallFunction|UpdateBuildingInstance))))

(fn IsWaterAhead
  (bind _returnvalue (Transformation|GetActorLocation))
  (bind _returnvalue_2 (Transformation|GetActorRotation))
  (bind _returnvalue_3 (Math|Vector|GetForwardVector _returnvalue_2))
  (bind _returnvalue_4 (Collision|SphereTraceForObjects (+ (* _returnvalue_3 5e+02) _returnvalue) (+ _returnvalue (* _returnvalue_3 1e+03)) 1e+02 (Utilities|Array|MakeArray "ObjectTypeQuery12") false 0 "None"))
  (return _returnvalue_4))

(fn FindSteeringSocket
  (Utilities|FlowControl|Sequence
    (:then_0
      (for _array_element (Actor|GetAttachedActors)
        (bind _asbp_ship_control_placeable (Utilities|Casting|CastToBP_ShipControlPlaceable _array_element))
        (if (Transformation|DoesSocketExist (Variables|/Game/Systems/Building/Placeables/BP_Master_Placeables.BP_Master_Placeables_C|GetStaticMesh _asbp_ship_control_placeable) "SteeringSocket")
          (return (Math|Transform|ComposeTransforms (Transformation|GetSocketTransform (Variables|/Game/Systems/Building/Placeables/BP_Master_Placeables.BP_Master_Placeables_C|GetStaticMesh _asbp_ship_control_placeable) "SteeringSocket" "RTS_World") (Math|Transform|InvertTransform (Transformation|GetActorTransform)))))))
    (:then_1
      (for _array_element_2 (Actor|GetComponentsByClass "/Script/Engine.InstancedStaticMeshComponent")
        (if (Transformation|DoesSocketExist _array_element_2 "SteeringSocket")
          (return (Math|Transform|ComposeTransforms (Transformation|GetSocketTransform _array_element_2 "SteeringSocket" "RTS_Actor") (.OutInstanceTransform (Components|InstancedStaticMesh|GetInstanceTransform _array_element_2 0 false))))))
      (return ""))))

(fn BobbingGetCurrentRotator
  (bind _bobbingcurrentvalue (Variables|Default|GetbobbingCurrentValue))
  (bind _bobbingconstraints (Variables|Default|GetbobbingConstraints))
  (bind _item (Utilities|Array|Get(acopy) _bobbingconstraints 1))
  (bind _item_2 (Utilities|Array|Get(acopy) _bobbingconstraints))
  (return (Math|Rotator|MakeRotator (Math|Interpolation|Ease "EaseInOut" (Utilities|Array|Get(acopy) _bobbingcurrentvalue) (- 0.0 _item_2) _item_2 2.0) (Math|Interpolation|Ease "EaseInOut" (Utilities|Array|Get(acopy) _bobbingcurrentvalue 1) (- 0.0 _item) _item 2.0) 0.0)))

(fn BobbingAdvanceValues
  (params (deltaTime :type Float%20%28single-precision%29))
  (bind _bobbingincrements (Variables|Default|GetbobbingIncrements))
  (LocalVariables|SetdeltaTimeVar deltaTime)
  (for (_array_element _array_index) (Variables|Default|GetbobbingCurrentValue)
    (Utilities|Array|SetArrayElem (Variables|Default|GetbobbingCurrentValue) _array_index (+ _array_element (* (Utilities|Array|Get(acopy) (Variables|Default|GetbobbingIncrements) _array_index) (LocalVariables|GetdeltaTimeVar))))
    (if (or (>= (+ _array_element (* (Utilities|Array|Get(acopy) (Variables|Default|GetbobbingIncrements) _array_index) (LocalVariables|GetdeltaTimeVar))) 1.0) (<= (+ _array_element (* (Utilities|Array|Get(acopy) (Variables|Default|GetbobbingIncrements) _array_index) (LocalVariables|GetdeltaTimeVar))) 0.0))
      (Utilities|Array|SetArrayElem _bobbingincrements _array_index (- 0.0 (Utilities|Array|Get(acopy) _bobbingincrements _array_index))))))

(fn ToggleWaterSplashParticles
  (params (newState :type Boolean))
  (bind _watersplashparticle (Variables|Default|GetWaterSplashParticle))
  (bind _returnvalue (Components|Activation|IsActive _watersplashparticle))
  (if newState
    (if (not _returnvalue)
      (Components|Activation|Activate (Variables|Default|GetWaterSplashParticle) false)
      (Components|Activation|Activate (Variables|Default|GetWaterSplashParticle2) false)
      (Components|Activation|Activate (Variables|Default|GetWaterSplashParticle3) false))
    (elif _returnvalue
      (Components|Activation|Deactivate (Variables|Default|GetWaterSplashParticle)))))

(fn CheckforOverlappingActors
  (bind _placeablecollisionbox (Variables|Default|GetPlaceableCollisionBox))
  (bind _returnvalue (Transformation|GetWorldLocation _placeablecollisionbox))
  (bind (_x _y _z) (Math|Vector|BreakVector _returnvalue))
  (bind _outhits (Class|KismetSystemLibrary|BoxTraceMultiforObjects _returnvalue (Math|Vector|MakeVector _x _y (- _z 1.0)) (Components|Box|GetScaledBoxExtent _placeablecollisionbox) (Transformation|GetWorldRotation _placeablecollisionbox) (Utilities|Array|MakeArray "ObjectTypeQuery2" "ObjectTypeQuery10" "ObjectTypeQuery3") false 0 "None" true))
  (for _array_element _outhits
    (Utilities|Array|Add (LocalVariables|GetoverlappingActorsFound) (.HitActor (Collision|BreakHitResult _array_element))))
  (return (LocalVariables|GetoverlappingActorsFound)))

(fn GetOverlappingObjects
  (params (box :type Box%20Component%20Object%20Reference) (types :type Array%20of%20EObjectTypeQuery%20Enums))
  (bind _returnvalue (Transformation|GetWorldLocation box))
  (bind (_x _y _z) (Math|Vector|BreakVector _returnvalue))
  (bind _outhits (Class|KismetSystemLibrary|BoxTraceMultiforObjects _returnvalue (Math|Vector|MakeVector _x _y (- _z 1.0)) (Components|Box|GetScaledBoxExtent box) (Transformation|GetWorldRotation box) types false 0 "None" true))
  (return _outhits))

(fn IsObstacle
  (params (actor :type Actor%20Object%20Reference))
  (Utilities|FlowControl|Sequence
    (:then_0
      (Utilities|Casting|CastToNavModifierVolume actor)
      (return false))
    (:then_1
      (if (== actor self)
        (return false)))
    (:then_2
      (return true))))

(fn IsAnyObstacle
  (params (actor :type Array%20of%20Actor%20Object%20References))
  (for _array_element actor
    (if (CallFunction|IsObstacle _array_element)
      (return true)))
  (return false))

(fn InteractableActivateDisabled
  (params (InteractingCharacter :type Conan%20Character%20Object%20Reference))
  (return false))

(fn InteractableCanbeLooted
  (params (InteractingCharacter :type Conan%20Character%20Object%20Reference))
  (return false))

(fn InteractableDefaultAction
  (return "" 0))

(fn InteractableGetRepairUIModuleName
  (return "None"))

(fn InteractableGetSimpleDisplayText
  (return ""))

(fn InteractableGetUIModuleName
  (return "None"))

(fn InteractableMenuDisabled
  (params (InteractingCharacter :type Conan%20Character%20Object%20Reference))
  (return false))

(fn InteractableShouldCommand
  (return false))