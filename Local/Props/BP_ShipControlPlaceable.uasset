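; Ship control placeable that lets players steer, launch or scuttle a boat through direct interaction or a radial menu.
; Client activation requests steering; the menu offers Steer and Scuttle when its placeable component has a ship, and Launch when a ship building is found.
; The ship building is detected by a sphere trace below the actor.
; All actions are forwarded as requests to the SOTE component on player controller 0.
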(event Custom|OnSteerClicked
  (params (menuEntry :type Radial%20Menu%20Entry%20Object%20Reference))
  ;[1 1 1] Steering
  (Default|ReqSteerShip (CallFunction|GetSOTEComp) (CallFunction|GetShip)))

(event Custom|OnLaunchClicked
  (params (menuEntry :type Radial%20Menu%20Entry%20Object%20Reference))
  ;[1 1 1] Launching
  (Default|ReqLaunchShip (CallFunction|GetSOTEComp) (CallFunction|GetShipBuilding)))

(event Custom|OnScuttleClicked
  (params (menuEntry :type Radial%20Menu%20Entry%20Object%20Reference))
  ;[1 1 1] Scuttling
  (Default|ReqScuttleShip (CallFunction|GetSOTEComp) (CallFunction|GetShip)))

(event EventInteractableActivate
  (params (Component :type Primitive%20Component%20Object%20Reference) (Instigator :type Player%20Controller%20Object%20Reference) (HitIndex :type Integer) (TriggeredFromRadialWheel :type Boolean)))

(event EventClientInteractableActivate
  (params (Component :type Primitive%20Component%20Object%20Reference) (Instigator :type Player%20Controller%20Object%20Reference) (HitIndex :type Integer))
  (CallFunction|OnSteerClicked))

(event EventInteractableMenu
  (params (RadialMenu :type Radial%20Menu%20Object%20Reference) (HitIndex :type Integer))
  (|CallParentFunction RadialMenu HitIndex)
  (Utilities|FlowControl|Sequence
    (:then_0
      ;[1 1 1] Steering
      (if (Utilities|IsValid (CallFunction|GetShip))
        (bind _returnvalue (Class|RadialMenu|AddItem RadialMenu "Steer" "Steer" "/Game/Mods/ShipsOfTheExiled/Icons/icon_wheel_1.icon_wheel_1" "None" -1))
        (EventDispatchers|BindEventtoSignalClicked _returnvalue (delegate Custom|OnSteerClicked))))
    (:then_1
      ;[1 1 1] Launching
      (if (Utilities|IsValid (CallFunction|GetShipBuilding))
        (bind _returnvalue_2 (Class|RadialMenu|AddItem RadialMenu "Launch Boat" "Launch Boat" "/Game/Mods/ShipsOfTheExiled/Icons/icon_khitanvessel.icon_khitanvessel" "None" -1))
        (EventDispatchers|BindEventtoSignalClicked _returnvalue_2 (delegate Custom|OnLaunchClicked))))
    (:then_2
      ;[1 1 1] Scuttling
      (if (Utilities|IsValid (CallFunction|GetShip))
        (bind _returnvalue_3 (Class|RadialMenu|AddItem RadialMenu "Scuttle Boat" "Scuttle Boat" "/Game/UI/Textures/FriendsIcons/T_DeleteButton_up.T_DeleteButton_up" "None" -1))
        (EventDispatchers|BindEventtoSignalClicked _returnvalue_3 (delegate Custom|OnScuttleClicked))))))

(fn ConstructionScript
  (|CallParentFunction))

(fn GetShip
  (return (Variables|/Game/Mods/ShipsOfTheExiled/System/SOTE_Placeable_AC.SOTE_Placeable_AC_C|Getship (Actor|GetComponentbyClass "/Game/Mods/ShipsOfTheExiled/System/SOTE_Placeable_AC.SOTE_Placeable_AC_C"))))

(fn GetShipBuilding
  (bind _returnvalue (Transformation|GetActorLocation))
  (bind _outhit (Collision|SphereTraceByChannel _returnvalue (- _returnvalue "0, 0,200.000000") 2e+02 "TraceTypeQuery3" false 0 "None"))
  (return (.AsBP%20Ship%20Building (Utilities|Casting|CastToBP_ShipBuilding (.HitActor (Collision|BreakHitResult _outhit))))))

(fn GetSOTEComp
  (return (Actor|GetComponentbyClass (Game|GetPlayerController 0) "/Game/Mods/ShipsOfTheExiled/System/SOTE_PC_AC.SOTE_PC_AC_C")))