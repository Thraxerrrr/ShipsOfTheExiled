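; BP_ShipInput handles player controls while steering a ship, acting on a steering character in a Conan Exiles setup.
; Movement follows control yaw, scaled by water and obstacle checks, while the mouse rotates and zooms the spring-arm camera.
; Left and right axes are paired into a clamped turn momentum that decays without input and drives yaw at state-dependent rates.
; Crouch exits steering only when horizontally stationary, otherwise showing a warning.
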(event Input|ActionEvents|InputActionCrouchMode
  (params (Key :type Key%20Structure :default "AnyKey"))
  (bind _steeringchar (Variables|Default|GetsteeringChar))
  (bind _returnvalue (Transformation|GetVelocity _steeringchar))
  ;[1 1 1] Crouch: exit steering
  (:Pressed
    (if (Math|Vector|Equal(Vector) (Math|Vector|MakeVector (.x _returnvalue) (.y _returnvalue) 0.0) "0,0.000000, 0" 0.0001)
      (Default|StopSteering (Actor|GetComponentbyClass (Variables|Default|GetsteeringChar) "/Game/Mods/ShipsOfTheExiled/System/BP_SteeringCharComp.BP_SteeringCharComp_C"))
      (else
        (Class|ConanPlayerController|ClientHUDShowNotification (.AsConan%20Player%20Controller (Utilities|Casting|CastToConanPlayerController (Pawn|GetController (Variables|Default|GetsteeringChar)))) (Utilities|Text|MakeLiteralText "Stop the boat before leaving control") false true)))))

(event Input|AxisEvents|InputAxisMoveLeft
  (params (AxisValue :type Float%20%28single-precision%29))
  ;[1 1 1] Axis movement
  (CallFunction|HandleTurnInput AxisValue true))

(event Input|AxisEvents|InputAxisMoveRight
  (params (AxisValue :type Float%20%28single-precision%29))
  ;[1 1 1] Axis movement
  (CallFunction|HandleTurnInput AxisValue false))

(event Input|AxisEvents|InputAxisMoveForward
  (params (AxisValue :type Float%20%28single-precision%29))
  ;[1 1 1] Axis movement
  (Pawn|Input|AddMovementInput (Variables|Default|GetsteeringChar) (CallFunction|GetCharOrientation) (* AxisValue (CallFunction|CalcForwardMovementFactor)) false))

(event Input|AxisEvents|InputAxisMoveBackwards
  (params (AxisValue :type Float%20%28single-precision%29))
  ;[1 1 1] Axis movement
  (Pawn|Input|AddMovementInput (Variables|Default|GetsteeringChar) (CallFunction|GetCharOrientation) (* AxisValue (CallFunction|CalcBackwardMovementFactor)) false))

(event Input|MouseEvents|MouseX
  (params (AxisValue :type Float%20%28single-precision%29))
  (bind _ship (Variables|Default|Getship))
  (bind _steeringcharcomp (Variables|/Game/Mods/ShipsOfTheExiled/Ships/BP_Ship.BP_Ship_C|GetsteeringCharComp _ship))
  (bind _steeringcameraspringarm (Variables|/Game/Mods/ShipsOfTheExiled/System/BP_SteeringCharComp.BP_SteeringCharComp_C|GetsteeringCameraSpringArm _steeringcharcomp))
  (bind _relativerotation (Variables|/Script/Engine.SceneComponent|GetRelativeRotation _steeringcameraspringarm))
  (bind (_roll _pitch _yaw) (Math|Rotator|BreakRotator _relativerotation))
  ;[1 1 1] Camera control
  (Transformation|AddLocalRotation _steeringcameraspringarm (Math|Rotator|MakeRotator 0.0 0.0 AxisValue) false false)
  (Transformation|SetRelativeRotation _steeringcameraspringarm (Math|Rotator|MakeRotator 0.0 _pitch _yaw) false false))

(event Input|MouseEvents|MouseY
  (params (AxisValue :type Float%20%28single-precision%29))
  (bind _ship (Variables|Default|Getship))
  (bind _steeringcharcomp (Variables|/Game/Mods/ShipsOfTheExiled/Ships/BP_Ship.BP_Ship_C|GetsteeringCharComp _ship))
  (bind _steeringcameraspringarm (Variables|/Game/Mods/ShipsOfTheExiled/System/BP_SteeringCharComp.BP_SteeringCharComp_C|GetsteeringCameraSpringArm _steeringcharcomp))
  (bind _relativerotation (Variables|/Script/Engine.SceneComponent|GetRelativeRotation _steeringcameraspringarm))
  (bind (_roll _pitch _yaw) (Math|Rotator|BreakRotator _relativerotation))
  ;[1 1 1] Camera control
  (Transformation|AddLocalRotation _steeringcameraspringarm (Math|Rotator|MakeRotator 0.0 AxisValue 0.0) false false)
  (Transformation|SetRelativeRotation _steeringcameraspringarm (Math|Rotator|MakeRotator 0.0 _pitch _yaw) false false))

(event Input|MouseEvents|MouseWheelAxis
  (params (AxisValue :type Float%20%28single-precision%29))
  (bind _ship (Variables|Default|Getship))
  (bind _steeringcharcomp (Variables|/Game/Mods/ShipsOfTheExiled/Ships/BP_Ship.BP_Ship_C|GetsteeringCharComp _ship))
  (bind _steeringcameraspringarm (Variables|/Game/Mods/ShipsOfTheExiled/System/BP_SteeringCharComp.BP_SteeringCharComp_C|GetsteeringCameraSpringArm _steeringcharcomp))
  ;[1 1 1] Camera control
  (Variables|/Script/Engine.SpringArmComponent|SetTargetArmLength _steeringcameraspringarm (- (Variables|/Script/Engine.SpringArmComponent|GetTargetArmLength _steeringcameraspringarm) (* AxisValue 3e+01))))

(fn ConstructionScript)

(fn GetCharOrientation
  (return (Math|Vector|GetForwardVector (Math|Rotator|MakeRotator 0.0 0.0 (.Yaw (Math|Rotator|BreakRotator (Pawn|GetControlRotation (Variables|Default|GetsteeringChar) :!class /Script/Engine.Pawn)))))))

(fn IsSwimming
  (return (Utilities|Enum|Equal(Enum) (Variables|/Script/Engine.CharacterMovementComponent|GetMovementMode (Variables|/Script/Engine.Character|GetCharacterMovement (Variables|Default|GetsteeringChar))) "MOVE_Swimming")))

(fn CalcForwardMovementFactor
  (bind _ship (Variables|Default|Getship))
  (if (and (or (CallFunction|IsSwimming) (Variables|/Game/Mods/ShipsOfTheExiled/Ships/BP_Ship.BP_Ship_C|GetoverlappingWater _ship)) (not (Variables|/Game/Mods/ShipsOfTheExiled/Ships/BP_Ship.BP_Ship_C|GetoverlapObstacleAhead _ship)))
    (return 1.0)
    (else
      (return 0.0))))

(fn CalcBackwardMovementFactor
  (if (not (Variables|/Game/Mods/ShipsOfTheExiled/Ships/BP_Ship.BP_Ship_C|GetoverlapObstacleBehind (Variables|Default|Getship)))
    (return 0.5)
    (else
      (return 0.0))))

(fn CalcTurnRateFactor
  (bind _ship (Variables|Default|Getship))
  (if (or (CallFunction|IsSwimming) (Variables|/Game/Mods/ShipsOfTheExiled/Ships/BP_Ship.BP_Ship_C|GetoverlappingWater (Variables|Default|Getship)))
    (if (> (Math|Float|Absolute(Float) (CallFunction|GetForwardVelocity (Variables|Default|GetsteeringChar))) 0.0)
      (return (Variables|/Game/Mods/ShipsOfTheExiled/Ships/BP_Ship.BP_Ship_C|GetshipControlTurnRate _ship))
      (else
        (return (Variables|/Game/Mods/ShipsOfTheExiled/Ships/BP_Ship.BP_Ship_C|GetshipControlTurnRateStatic _ship))))
    (else
      (return (* (Variables|/Game/Mods/ShipsOfTheExiled/Ships/BP_Ship.BP_Ship_C|GetshipControlTurnRate (Variables|Default|Getship)) 0.3)))))

(fn HandleTurnInput
  (params (input :type Float%20%28single-precision%29) (isLeftInput :type Boolean))
  (Utilities|FlowControl|Sequence
    (:then_0
      (if isLeftInput
        (Variables|Default|SetturnInputLeft input)
        (else
          (Variables|Default|SetturnInputRight input))))
    (:then_1
      ;[1 1 1] If both inputs have been received, update the turn impact
      (if (and (!= (Variables|Default|GetturnInputLeft) 1e+03) (!= (Variables|Default|GetturnInputRight) 1e+03))
        (Utilities|FlowControl|Sequence
          (:then_0
            (if (!= (Variables|Default|GetturnInputLeft) 0.0)
              (LocalVariables|SetturnInput (Variables|Default|GetturnInputLeft))))
          (:then_1
            (if (!= (Variables|Default|GetturnInputRight) 0.0)
              (LocalVariables|SetturnInput (Variables|Default|GetturnInputRight))))
          (:then_2
            (if (== (LocalVariables|GetturnInput) 0.0)
              (if (!= (Variables|Default|GetturnImpact) 0.0)
                ;[1 1 1] No input: reduce impact towards zero
                (bind _output_get (Variables|Default|SetturnImpact (- (Variables|Default|GetturnImpact) (* (Utilities|Time|GetWorldDeltaSeconds) (/ (Variables|Default|GetturnImpact) (Math|Float|Absolute(Float) (Variables|Default|GetturnImpact))) 2.0))))
                (if (< (Math|Float|Absolute(Float) _output_get) 0.001)
                  (Variables|Default|SetturnImpact 0.0)))
              (else
                (if (< (CallFunction|GetForwardVelocity (Variables|Default|GetsteeringChar)) 0.0)
                  (Math|Float|NegateFloat (LocalVariables|GetturnInput)
                    (:%20%20
                      _)))
                ;[1 1 1] Input received: increase turn impact
                (Variables|Default|SetturnImpact (Math|Float|Clamp(Float) (+ (Variables|Default|GetturnImpact) (* (Utilities|Time|GetWorldDeltaSeconds) (LocalVariables|GetturnInput))) -8.0 8.0)))))
          (:then_3
            ;[1 1 1] Apply the calculated turn impact
            (Pawn|Input|AddControllerYawInput (Variables|Default|GetsteeringChar) (* (Utilities|Time|GetWorldDeltaSeconds) (Variables|Default|GetturnImpact) (CallFunction|CalcTurnRateFactor)))
            (Variables|Default|SetturnInputLeft 1e+03)
            (Variables|Default|SetturnInputRight 1e+03)))))))