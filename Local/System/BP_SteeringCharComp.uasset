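; Player character component for steering a BP_Ship by attaching the ship to the character, whose retuned swimming and buoyancy movement carries it.
; Setting or clearing the Ship RepNotify starts or stops steering, adjusting capsule collision and posing the mesh at the ship's steering socket.
; The owning client gets a spring-arm camera, HUD and spawned BP_ShipInput actor.
; On exit, a delayed multicast restores the ship's position, working around a client teleport bug.
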(event Custom|startSteering
  (params (ship :type BP%20Ship%20Object%20Reference))
  ;[1 1 1] Steering: server RPCs
  (Variables|Default|Setship ship))

(event Custom|doStopSteering
  (Utilities|FlowControl|Sequence
    (:then_0
      ;[1 1 1] Detach the ship
      (for _array_element (Actor|GetAttachedActors (Variables|Default|GetsteeringChar))
        (bind _asbp_ship (Utilities|Casting|CastToBP_Ship _array_element))
        (Variables|/Game/Mods/ShipsOfTheExiled/Ships/BP_Ship.BP_Ship_C|SetsteeringCharComp _asbp_ship 0)
        (Transformation|DetachFromActor _asbp_ship "KeepWorld" "KeepWorld" "KeepWorld")))
    (:then_1
      ;[1 1 1] Reposition steering char
      (Transformation|SetRelativeTransform (Variables|/Script/Engine.Character|GetMesh (Variables|Default|GetsteeringChar)) (Math|Transform|MakeTransform "0,0.000000,-96.000000" "0.000000,-90.000000,0.000000") false true)
      (Transformation|SetActorTransform (Variables|Default|GetsteeringChar) (Math|Transform|ComposeTransforms (Math|Transform|ComposeTransforms (Variables|Default|GetsteeringPosition) (Math|Conversions|ToTransform(Vector) "0, 0,100.000000")) (Transformation|GetActorTransform (Variables|Default|GetsteeringChar))) false true)
      (CallFunction|ResetSteeringCharCollision)
      (CallFunction|PlaySteeringAnimation))
    (:then_2
      (if (CallFunction|IsOwningClient)
        (CallFunction|ClearSteeringCharMovementSettings)
        (CallFunction|DisableSteeringInput)
        (CallFunction|RemoveSteeringCamera)
        (CallFunction|ToggleSteeringHUD false)))
    (:then_3
      (if (Networking|IsServer)
        ;[1 1 1] Workaround for weird client issue where ship teleports far away when exiting
        (Utilities|FlowControl|Delay 1.0)
        (CallFunction|MulticastRepositionShip (Variables|Default|GetstoppedPosition) _asbp_ship)))))

(event Custom|createSteeringCamera
  (bind _ship (Variables|Default|Getship))
  (Utilities|IsValid+Branch (Variables|Default|GetsteeringCameraSpringArm) true
    (:True
      _)
    (:False%20or%20Invalid
      (bind _returnvalue (Class|FuncomGenericLibrary|AddComponentbyClass (Variables|Default|GetsteeringChar) "/Script/Engine.SpringArmComponent" (Math|Conversions|ToTransform(Vector) "0, 0, 0")))
      (bind _asspring_arm_component (Utilities|Casting|CastToSpringArmComponent _returnvalue))
      (bind _output_get (Variables|Default|SetsteeringCameraSpringArm _asspring_arm_component))
      (Variables|/Script/Engine.SpringArmComponent|SetbDoCollisionTest _output_get false)
      (bind _returnvalue_2 (Class|FuncomGenericLibrary|AddComponentbyClass (Variables|Default|GetsteeringChar) "/Script/Engine.CameraComponent" (Math|Conversions|ToTransform(Vector) "0, 0, 0")))
      (bind _ascamera_component (Utilities|Casting|CastToCameraComponent _returnvalue_2))
      (bind _output_get_2 (Variables|Default|SetsteeringCamera _ascamera_component))
      (Transformation|AttachComponentToComponent _output_get_2 (Variables|Default|GetsteeringCameraSpringArm) "None" "KeepRelative" "KeepRelative" "KeepRelative" true)))
  (Variables|/Script/Engine.SpringArmComponent|SetTargetArmLength (Variables|Default|GetsteeringCameraSpringArm) (Variables|/Game/Mods/ShipsOfTheExiled/Ships/BP_Ship.BP_Ship_C|GetshipCameraDistance _ship))
  (Variables|/Script/Engine.SpringArmComponent|SetSocketOffset (Variables|Default|GetsteeringCameraSpringArm) (Math|Vector|MakeVector 0.0 0.0 (Variables|/Game/Mods/ShipsOfTheExiled/Ships/BP_Ship.BP_Ship_C|GetshipCameraHeight _ship)))
  (Default|SwitchtoThirdPersonCamera (Variables|Default|GetsteeringChar))
  (Components|Activation|Activate (Variables|Default|GetsteeringCamera) false)
  (Components|Activation|Deactivate (Variables|/Game/Characters/BasePlayerChar.BasePlayerChar_C|GetCameraThirdPerson (Variables|Default|GetsteeringChar))))

(event Custom|removeSteeringCamera
  (Default|SwitchtoThirdPersonCamera (Variables|Default|GetsteeringChar))
  (Components|Activation|Deactivate (Variables|Default|GetsteeringCamera)))

(event Custom|doStartSteering
  (bind _returnvalue (Math|Transform|MakeTransform "0,0.000000,-96.000000" "0.000000,-90.000000,0.000000"))
  (bind _ship (Variables|Default|Getship))
  (bind _transform (Default|FindSteeringSocket _ship))
  (bind _returnvalue_2 (Math|Transform|ComposeTransforms _returnvalue _transform))
  (Utilities|FlowControl|Sequence
    (:then_0
      (if (CallFunction|IsOwningClient)
        (CallFunction|ApplySteeringCharMovementSettings)
        (CallFunction|EnableSteeringInput)
        (CallFunction|CreateSteeringCamera)
        (CallFunction|ToggleSteeringHUD true)))
    (:then_1
      (if (or (CallFunction|IsOwningClient) (Networking|IsServer))
        ;[1 1 1] Position steering char
        (Components|Movement|StopMovementImmediately (Variables|/Script/Engine.Character|GetCharacterMovement (Variables|Default|GetsteeringChar)))
        (Pawn|SetControlRotation (Pawn|GetController (Variables|Default|GetsteeringChar)) (Transformation|GetActorRotation (Variables|Default|Getship)))
        (Transformation|SetActorTransform (Variables|Default|GetsteeringChar) (Transformation|GetActorTransform (Variables|Default|Getship)) false true)))
    (:then_2
      (CallFunction|ConfigureSteeringCharCollision)
      ;[1 1 1] Attach ship to steering char
      (Transformation|AttachActorToActor (Variables|Default|Getship) (Variables|Default|GetsteeringChar) "None" "KeepWorld" "KeepWorld" "KeepWorld" true)
      (Variables|/Game/Mods/ShipsOfTheExiled/Ships/BP_Ship.BP_Ship_C|SetsteeringCharComp (Variables|Default|Getship) self)
      ;[1 1 1] Configure steering char visuals
      (Variables|Default|SetsteeringPosition (Math|Transform|MakeTransform (.location _returnvalue_2) (.rotation _returnvalue_2) "1.000000,1.000000,1"))
      (if (Variables|/Game/Mods/ShipsOfTheExiled/Ships/BP_Ship.BP_Ship_C|GetbobbingEnabled (Variables|Default|Getship))
        _
        (else
          (CallFunction|RepositionSteeringChar "0, 0, 0")))
      (CallFunction|PlaySteeringAnimation))))

(event Custom|enableSteeringInput
  (Input|DisableInput (Variables|Default|GetsteeringChar) 0)
  (bind _returnvalue (Game|SpawnActorfromClass "/Game/Mods/ShipsOfTheExiled/System/BP_ShipInput.BP_ShipInput_C" (Transformation|GetActorTransform (Variables|Default|Getship)) "Undefined" 0 0))
  (bind _output_get (Variables|Default|SetshipInput _returnvalue))
  (Transformation|AttachActorToActor _output_get (Variables|Default|GetsteeringChar) "None" "KeepWorld" "KeepWorld" "KeepWorld" true)
  (Variables|/Game/Mods/ShipsOfTheExiled/System/BP_ShipInput.BP_ShipInput_C|Setship (Variables|Default|GetshipInput) (Variables|Default|Getship))
  (Variables|/Game/Mods/ShipsOfTheExiled/System/BP_ShipInput.BP_ShipInput_C|SetsteeringChar (Variables|Default|GetshipInput) (Variables|Default|GetsteeringChar))
  (Input|EnableInput (Variables|Default|GetshipInput) (.AsPlayer%20Controller (Utilities|Casting|CastToPlayerController (Pawn|GetController (Variables|Default|GetsteeringChar))))))

(event Custom|disableSteeringInput
  (Input|EnableInput (Variables|Default|GetsteeringChar) 0)
  (Actor|DestroyActor (Variables|Default|GetshipInput)))

(event Custom|applySteeringCharMovementSettings
  (bind _steeringchar (Variables|Default|GetsteeringChar))
  (bind _charactermovement (Variables|/Script/Engine.Character|GetCharacterMovement _steeringchar))
  (Variables|/Script/Engine.CharacterMovementComponent|SetMaxAcceleration _charactermovement 128.0)
  (Variables|/Script/Engine.CharacterMovementComponent|SetbDisableBuoyancy _charactermovement false)
  (Variables|/Script/Engine.CharacterMovementComponent|SetOutofWaterZ _charactermovement 1e+01)
  (Variables|/Script/Engine.CharacterMovementComponent|SetBuoyancy _charactermovement 2.0)
  (Variables|/Script/Engine.CharacterMovementComponent|SetBrakingDecelerationSwimming _charactermovement 5e+01)
  (Variables|/Script/Engine.CharacterMovementComponent|SetMaxSwimSpeed _charactermovement (Variables|/Game/Mods/ShipsOfTheExiled/Ships/BP_Ship.BP_Ship_C|GetshipControlMaxSpeed (Variables|Default|Getship)))
  (Variables|/Script/Engine.CharacterMovementComponent|SetbOrientRotationToMovement _charactermovement false)
  (Variables|/Script/Engine.CharacterMovementComponent|SetbUseControllerDesiredRotation _charactermovement false))

(event Custom|repositionSteeringChar
  (params (bobbingRotator :type Rotator))
  (Transformation|SetRelativeTransform (Variables|/Script/Engine.Character|GetMesh (Variables|Default|GetsteeringChar)) (Math|Transform|ComposeTransforms (Variables|Default|GetsteeringPosition) (Math|Transform|MakeTransform "0, 0, 0" bobbingRotator)) false true))

(event Custom|stopSteering
  ;[1 1 1] Steering: server RPCs
  (Variables|Default|SetstoppedPosition (Transformation|GetActorTransform (Variables|Default|Getship)))
  (Variables|Default|Setship 0))

(event Custom|playSteeringAnimation
  (bind _ship (Variables|Default|Getship))
  (bind _ship_2 (Variables|Default|Getship))
  (bind _steeringchar (Variables|Default|GetsteeringChar))
  (bind _mesh (Variables|/Script/Engine.Character|GetMesh _steeringchar))
  (Utilities|IsValid+Branch _ship_2 true
    (:True
      (Utilities|IsValid+Branch (Variables|/Game/Mods/ShipsOfTheExiled/Ships/BP_Ship.BP_Ship_C|GetsteeringAnim _ship_2) true
        (:True
          (Components|Animation|PlayAnimation _mesh (Variables|/Game/Mods/ShipsOfTheExiled/Ships/BP_Ship.BP_Ship_C|GetsteeringAnim (Variables|Default|Getship)) true)
          (Utilities|FlowControl|Delay 2.0) ; Trigger twice: for clients that enter render range the char will lie sleeping because it's considered unconscious
          (Utilities|IsValid+Branch _ship true
            (:True
              (Components|Animation|PlayAnimation _mesh (Variables|/Game/Mods/ShipsOfTheExiled/Ships/BP_Ship.BP_Ship_C|GetsteeringAnim _ship) true))))
        (:False%20or%20Invalid
          (Components|Animation|SetAnimationMode _mesh "AnimationBlueprint" :!label _label))))
    (:False%20or%20Invalid
      (goto _label))))

(event Custom|configureSteeringCharCollision
  (bind _steeringchar (Variables|Default|GetsteeringChar))
  (bind _capsulecomponent (Variables|/Script/Engine.Character|GetCapsuleComponent _steeringchar))
  (Variables|/Script/Engine.Pawn|SetbUseControllerRotationYaw (Variables|Default|GetsteeringChar) true)
  (Components|Capsule|SetCapsuleHalfHeight _capsulecomponent 4e+01 true)
  (Components|Capsule|SetCapsuleRadius _capsulecomponent 34.0 true)
  (Collision|IgnoreActorwhenMoving _capsulecomponent (Variables|Default|Getship) true))

(event Custom|MulticastRepositionShip
  (params (position :type Transform) (ship :type BP%20Ship%20Object%20Reference))
  ;[1 1 1] Workaround for weird client issue where ship teleports far away when exiting
  (Transformation|SetActorTransform ship position false true))

(event Custom|resetSteeringCharCollision
  (bind _steeringchar (Variables|Default|GetsteeringChar))
  (bind _capsulecomponent (Variables|/Script/Engine.Character|GetCapsuleComponent _steeringchar))
  (Variables|/Script/Engine.Pawn|SetbUseControllerRotationYaw (Variables|Default|GetsteeringChar) false)
  (Components|Capsule|SetCapsuleHalfHeight _capsulecomponent 96.0 true)
  (Components|Capsule|SetCapsuleRadius _capsulecomponent 42.0 true)
  (Collision|ClearMoveIgnoreActors _capsulecomponent))

(event Custom|toggleSteeringHUD
  (params (show :type Boolean))
  (if (CallFunction|IsOwningClient)
    (bind _windowroot (|GUIModuleControllerActivate (Class|GUIModuleController|GetGUIModuleController) "SOTE_SteeringInfo" show false)
      (:OnActivate
        (if show
          (Default|InitUI (.AsW%20Steering%20Info (Utilities|Casting|CastToW_SteeringInfo _windowroot)) (Variables|Default|Getship)))))))

(event Custom|clearSteeringCharMovementSettings
  (bind _steeringchar (Variables|Default|GetsteeringChar))
  (bind _charactermovement (Variables|/Script/Engine.Character|GetCharacterMovement _steeringchar))
  (Variables|/Script/Engine.CharacterMovementComponent|SetMaxAcceleration _charactermovement 1536.0)
  (Variables|/Script/Engine.CharacterMovementComponent|SetbDisableBuoyancy _charactermovement true)
  (Variables|/Script/Engine.CharacterMovementComponent|SetOutofWaterZ _charactermovement 5e+02)
  (Variables|/Script/Engine.CharacterMovementComponent|SetBuoyancy _charactermovement 1.6)
  (Variables|/Script/Engine.CharacterMovementComponent|SetBrakingDecelerationSwimming _charactermovement 7e+02)
  (Variables|/Script/Engine.CharacterMovementComponent|SetMaxSwimSpeed _charactermovement 3.5e+02)
  (Variables|/Script/Engine.CharacterMovementComponent|SetbOrientRotationToMovement _charactermovement true)
  (Variables|/Script/Engine.CharacterMovementComponent|SetbUseControllerDesiredRotation _charactermovement false))

(event EventEndPlay
  (params (EndPlayReason :type EEndPlayReason%20Enum :default "Destroyed"))
  (CallFunction|StopSteering))

(event EventBeginPlay
  (Variables|Default|SetsteeringChar (.AsBase%20Player%20Char (Utilities|Casting|CastToBasePlayerChar (Components|GetOwner)))))

(event EventTick
  (params (DeltaSeconds :type Float%20%28single-precision%29))
  (if (Utilities|IsValid (Variables|Default|Getship))
    (CallFunction|ApplySteeringCharMovementSettings)
    (if (not (Variables|/Game/Mods/ShipsOfTheExiled/Ships/BP_Ship.BP_Ship_C|GetbobbingEnabled (Variables|Default|Getship)))
      (CallFunction|RepositionSteeringChar "0, 0, 0"))))

(fn OnRepShip
  (if (Utilities|IsValid (Variables|Default|Getship))
    (CallFunction|DoStartSteering)
    (else
      (CallFunction|DoStopSteering))))

(fn IsOwningClient
  (return (and (not (Networking|IsDedicatedServer)) (== (Pawn|GetController (Variables|Default|GetsteeringChar)) (Game|GetPlayerController 0)))))