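; Component for characters riding a ship, keeping them moving with it until they are no longer standing on it.
; The Ship RepNotify makes the character follow base rotation and, for NPCs only, attaches it to the ship's mesh.
; A looping server timer traces downward for the ship; on a miss or different hit, it detaches NPCs and destroys the component.
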(event Custom|CheckStillOnShip
  (bind _returnvalue (Components|GetOwner))
  (bind _returnvalue_2 (Transformation|GetActorLocation _returnvalue))
  (bind (_outhit _returnvalue_3) (Collision|LineTraceForObjects _returnvalue_2 (+ _returnvalue_2 "0.000000, 0,-500.000000") (Utilities|Array|MakeArray "ObjectTypeQuery10") false 0 "None"))
  (if _returnvalue_3
    (if (not (== (Variables|Default|Getship) (.HitActor (Collision|BreakHitResult _outhit))))
      (CallFunction|DoLeaveShip :!label _label))
    (else
      (goto _label))))

(event Custom|DoEnterShip
  (bind _returnvalue (Components|GetOwner))
  (bind _asbase_bpchar (Utilities|Casting|CastToBaseBPChar _returnvalue))
  (Variables|/Script/Engine.CharacterMovementComponent|SetbIgnoreBaseRotation (Variables|/Script/Engine.Character|GetCharacterMovement _asbase_bpchar) false)
  (bind _asbase_npc (Utilities|Casting|CastToBaseNPC _asbase_bpchar))
  (Transformation|AttachComponentToComponent _asbase_npc (Variables|/Game/Mods/ShipsOfTheExiled/Ships/BP_Ship.BP_Ship_C|GetMesh (Variables|Default|Getship)) "" "KeepWorld" "KeepWorld" "KeepWorld" true))

(event Custom|DoLeaveShip
  (Utilities|FlowControl|Sequence
    (:then_0
      (bind _asbase_npc (Utilities|Casting|CastToBaseNPC (Components|GetOwner)))
      (Transformation|DetachFromActor _asbase_npc "KeepWorld" "KeepWorld" "KeepWorld"))
    (:then_1
      (Components|DestroyComponent))))

(event EventBeginPlay
  (if (Networking|IsServer)
    (Utilities|Time|SetTimerbyEvent (delegate Custom|CheckStillOnShip) 5.0 true)))

(fn OnRepShip
  (CallFunction|DoEnterShip))